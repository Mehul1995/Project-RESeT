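; BP_Fox is a fox actor that follows the VR player, stopping when it gets close to the MotionControllerPawn camera.
; Tick moves and yaws it by forward and turn speeds, then recomputes both from the camera's position.
; Yaw is a smoothed per-frame fraction of the look-at delta; speed interpolates to max or zero by 2D distance, with a half-speed step left unwired.
; Forward speed, as a percentage of max, sets the AnimMoveForward value.
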(event `self.ReceiveTick`
  (params (DeltaSeconds :type "Float (single-precision)"))
  (`self.K2_AddActorLocalOffset` (`KismetMathLibrary.MakeVector` (* (`self.FowardSpeed`) (`GameplayStatics.GetWorldDeltaSeconds`) 100.0)))
  (`self.K2_AddActorLocalRotation` (`KismetMathLibrary.MakeRotator` 0.0 0.0 (`self.TurnSpeed`)))
  (`self.TurnTowardsPlayer` 15.0)
  (`self.SpeedTowardsPlayer` 100.0 8.0)
  (set `self.AnimMoveForward` (* (/ (`self.FowardSpeed`) (`self.MaxSpeed`)) 100.0))
  (set `self.AnimMoveSide` 0.0))

(fn `SpeedTowardsPlayer`
  (params (Distance :type "Float (double-precision)" :default 500.0) (`Stop Speed` :type "Float (double-precision)" :default 2.0))
  (bind _asmotion_controller_pawn (cast `/Game/VirtualRealityBP/Blueprints/MotionControllerPawn` (`GameplayStatics.GetPlayerPawn` 0)))
  (`|ExecutionSequence`
    (:`then_0`
      (if (< (`KismetMathLibrary.Vector_Distance2D` (`self.K2_GetActorLocation`) (`SceneComponent.K2_GetComponentLocation` (`/Game/VirtualRealityBP/Blueprints/MotionControllerPawn.Camera` _asmotion_controller_pawn))) Distance)
        (set `self.TargetSpeed` 0.0)
        (else
          (if (< (/ Distance 2.0) Distance)
            _
            (else
              _))
          (set `self.TargetSpeed` (`self.MaxSpeed`)))))
    (:`then_1`
      (set `self.FowardSpeed` (`KismetMathLibrary.FInterpTo` (`self.FowardSpeed`) (`self.TargetSpeed`) (`GameplayStatics.GetWorldDeltaSeconds`) `Stop Speed`)))))

(fn `TurnTowardsPlayer`
  (params (Smoothing :type "Float (double-precision)" :default 7.0))
  (bind _asmotion_controller_pawn (cast `/Game/VirtualRealityBP/Blueprints/MotionControllerPawn` (`GameplayStatics.GetPlayerPawn` 0)))
  (bind _result (`/Engine/EditorBlueprintResources/StandardMacros.NegateFloat` (/ (.yaw (`KismetMathLibrary.NormalizedDeltaRotator` (`self.K2_GetActorRotation`) (`KismetMathLibrary.FindLookAtRotation` (`self.K2_GetActorLocation`) (`SceneComponent.K2_GetComponentLocation` (`/Game/VirtualRealityBP/Blueprints/MotionControllerPawn.Camera` _asmotion_controller_pawn))))) Smoothing))
    (:`  `
      (set `self.TurnSpeed` _result))))

(fn `UserConstructionScript`)