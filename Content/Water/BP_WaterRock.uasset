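; BP_WaterRock is a physics rock that BP_MotionController can pick up and throw, with a text label set at construction.
; Pickup turns off physics and attaches the root to the given component; Drop re-enables physics and detaches it.
; Tick tracks position change multiplied by delta time and debug-prints it.
; Drop adds that value, scaled by VelocityMultiplier, to the mesh's velocity.
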(event `self.ReceiveTick`
  (params (DeltaSeconds :type "Float (single-precision)"))
  (bind _returnvalue (`SceneComponent.K2_GetComponentLocation` (`self.StaticMesh`)))
  (bind _output_get (set `self.vel` (* (- _returnvalue (`self.lastpos`)) DeltaSeconds)))
  (set `self.lastpos` _returnvalue)
  (`KismetSystemLibrary.PrintString` (`KismetStringLibrary.Conv_VectorToString` _output_get) true true (struct :`G` 0.66 :`B` 1.0 :`A` 1.0) DeltaSeconds))

(event `/Game/VirtualRealityBP/Blueprints/PickupActorInterface.Pickup`
  (params (AttachTo :type "SceneComponent Object Reference"))
  (set `self.isheld` true)
  (`PrimitiveComponent.SetSimulatePhysics` (`self.StaticMesh`) false)
  (`SceneComponent.K2_AttachToComponent` (`self.K2_GetRootComponent`) AttachTo "None" "KeepWorld" "KeepWorld" "KeepWorld" false))

(event `/Game/VirtualRealityBP/Blueprints/PickupActorInterface.Drop`
  (set `self.isheld` false)
  (`PrimitiveComponent.SetSimulatePhysics` (`self.StaticMesh`) true)
  (`self.K2_DetachFromActor` "KeepWorld" "KeepWorld" "KeepWorld")
  (`PrimitiveComponent.SetAllPhysicsLinearVelocity` (`self.StaticMesh`) (* (`self.vel`) (`self.velocity multiplier`)) true))

(fn `UserConstructionScript`
  (`TextRenderComponent.K2_SetText` (`self.Text`) (`KismetTextLibrary.Conv_StringToText` (`self.TextContent`))))